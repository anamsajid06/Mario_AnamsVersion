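; Player controller for a Mario game that owns the player's HUD, lost screen and pause menu widgets.
; On BeginPlay it shows the HUD, and each widget is created on first use and cached in a reference.
; The lost screen event waits, shows its widget, pauses the game, then after another delay reopens the current level.
; The pause menu event switches to UI-only input and shows the mouse cursor, without pausing the game itself.
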(event EventBeginPlay
  (CallFunction|CreateHUD))

(event EventCreateLostScreen
  ;[1 1 1] Create lost widget, restart level
  (Utilities|FlowControl|Delay 2.0)
  (Utilities|IsValid (Variables|Default|GetLostMenuREF)
    (:Is%20Valid
      _)
    (:Is%20Not%20Valid
      (bind _returnvalue (UserInterface|CreateWidget "/Game/Mario/Blueprints/Widgets/BP_Lost.BP_Lost_C" self))
      (Variables|Default|SetLostMenuREF _returnvalue)))
  (UserInterface|Viewport|AddtoViewport (Variables|Default|GetLostMenuREF) 0)
  (Game|SetGamePaused true)
  (Utilities|FlowControl|Delay 2.0)
  (bind _returnvalue_2 (Game|GetCurrentLevelName true))
  (Game|OpenLevel(byName) (Utilities|String|StringToName _returnvalue_2)))

(event EventCreatePauseScreen
  ;[1 1 1] Create pause menu
  (Utilities|IsValid (Variables|Default|GetPauseMenuREF)
    (:Is%20Valid
      _)
    (:Is%20Not%20Valid
      (bind _returnvalue (UserInterface|CreateWidget "/Game/Mario/Blueprints/Widgets/BP_PauseMenu.BP_PauseMenu_C" self))
      (Variables|Default|SetPauseMenuREF _returnvalue)))
  (UserInterface|Viewport|AddtoViewport (Variables|Default|GetPauseMenuREF) 0)
  (Input|SetInputModeUIOnly self (Variables|Default|GetPauseMenuREF) "DoNotLock")
  (Variables|Default|SetbShowMouseCursor true))

(event EventCreateHUD
  ;[1 1 1] Create HUD
  (Utilities|IsValid (Variables|Default|GetHUDREF)
    (:Is%20Valid
      _)
    (:Is%20Not%20Valid
      (bind _returnvalue (UserInterface|CreateWidget "/Game/Mario/Blueprints/Widgets/BP_HUD.BP_HUD_C" self))
      (Variables|Default|SetHUDREF _returnvalue)))
  (UserInterface|Viewport|AddtoViewport (Variables|Default|GetHUDREF) 0))

(fn ConstructionScript)