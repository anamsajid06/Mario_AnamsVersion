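; Koopa enemy Character for a Mario-style game that patrols back and forth along the Y axis while looping a walk animation.
; Tick drives movement input, and each Hit event flip-flops the direction and mesh facing.
; A player overlapping the top box triggers death: collision boxes removed, give-up animation, squashed capsule, then destruction.
; Side-box overlap damages the player; a small player also gets the lost widget and a delayed level reload.
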(event OnComponentBeginOverlap(BoxCollisionTop)
  (params (OverlappedComponent :type Primitive%20Component%20Object%20Reference) (OtherActor :type Actor%20Object%20Reference) (OtherComp :type Primitive%20Component%20Object%20Reference) (OtherBodyIndex :type Integer) (bFromSweep :type Boolean) (SweepResult :type Hit%20Result%20Structure%20%28by%20ref%29))
  ;[1 1 1] Death
  (Utilities|EnemyDeath OtherActor))

(event OnComponentBeginOverlap(BoxCollisionSide)
  (params (OverlappedComponent :type Primitive%20Component%20Object%20Reference) (OtherActor :type Actor%20Object%20Reference) (OtherComp :type Primitive%20Component%20Object%20Reference) (OtherBodyIndex :type Integer) (bFromSweep :type Boolean) (SweepResult :type Hit%20Result%20Structure%20%28by%20ref%29))
  ;[1 1 1] Cause Damage to Player
  (bind _asbp_third_person_character (Utilities|Casting|CastToBP_ThirdPersonCharacter OtherActor))
  (Utilities|FlowControl|Sequence
    (:then_0
      (if (Variables|/Game/ThirdPerson/Blueprints/BP_ThirdPersonCharacter.BP_ThirdPersonCharacter_C|GetbIsBig _asbp_third_person_character)
        (Development|PrintString (Utilities|String|ToString(Boolean) (Variables|/Game/ThirdPerson/Blueprints/BP_ThirdPersonCharacter.BP_ThirdPersonCharacter_C|GetbIsBig _asbp_third_person_character)))
        (else
          (Development|PrintString (Utilities|String|ToString(Boolean) (Variables|/Game/ThirdPerson/Blueprints/BP_ThirdPersonCharacter.BP_ThirdPersonCharacter_C|GetbIsBig _asbp_third_person_character)))
          ;[1 1 1] Lost Widget
          (bind _returnvalue (UserInterface|CreateWidget "/Game/Mario/Blueprints/BP_Lost.BP_Lost_C"))
          (UserInterface|Viewport|AddtoViewport _returnvalue 0)
          (Utilities|FlowControl|Delay 3.0)
          (bind _returnvalue_2 (Game|GetCurrentLevelName true))
          (Game|OpenLevel(byName) (Utilities|String|StringToName _returnvalue_2)))))
    (:then_1
      (Default|DealDamage _asbp_third_person_character))))

(event EventBeginPlay
  ;[1 1 1] Walk Animation
  (Components|Animation|PlayAnimation (Variables|Character|GetMesh) "/Game/Mario/Assets/Koopa/Animations/Walk.Walk" true))

(event EventTick
  (params (DeltaSeconds :type Float%20%28single-precision%29))
  ;[1 1 1] Movement
  (Pawn|Input|AddMovementInput (Variables|Default|GetWorld%20Direction) 0.1 false))

(event Collision|EventHit
  (params (MyComp :type Primitive%20Component%20Object%20Reference) (Other :type Actor%20Object%20Reference) (OtherComp :type Primitive%20Component%20Object%20Reference) (bSelfMoved :type Boolean) (HitLocation :type Vector :default "0, 0, 0") (HitNormal :type Vector :default "0, 0, 0") (NormalImpulse :type Vector :default "0, 0, 0") (Hit :type Hit%20Result%20Structure%20%28by%20ref%29))
  ;[1 1 1] Change Direction on Hit
  (Utilities|FlowControl|FlipFlop
    (:A
      (Variables|Default|SetWorld%20Direction "0,1.000000, 0")
      (Transformation|SetRelativeRotation (Variables|Character|GetMesh) (Math|Rotator|MakeRotator 0.0 0.0 0.0) false false))
    (:B
      (Variables|Default|SetWorld%20Direction "0,-1.000000, 0")
      (Transformation|SetRelativeRotation (Variables|Character|GetMesh) "0,180.000000, 0" false false))))

(fn ConstructionScript)