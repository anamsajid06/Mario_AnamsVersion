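; BP_ShotObj is a shot object in a Mario game that kills enemies it touches.
; SphereCollision overlaps destroy a BP_Enemy or BP_Koopa along with the shot, while touching the player character only prints a debug string.
; A shot that hits no enemy destroys itself after a short delay from BeginPlay.
; The graph applies no motion, as its AddImpulse node is unconnected.
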(event OnComponentBeginOverlap(SphereCollision)
  (params (OverlappedComponent :type Primitive%20Component%20Object%20Reference) (OtherActor :type Actor%20Object%20Reference) (OtherComp :type Primitive%20Component%20Object%20Reference) (OtherBodyIndex :type Integer) (bFromSweep :type Boolean) (SweepResult :type Hit%20Result%20Structure%20%28by%20ref%29))
  ;[1 1 1] Destroy Enemies
  (bind _asbp_enemy (Utilities|Casting|CastToBP_Enemy OtherActor)
    (:then
      (Actor|DestroyActor _asbp_enemy)
      (Actor|DestroyActor :!label _label))
    (:CastFailed
      (Utilities|Casting|CastToBP_ThirdPersonCharacter OtherActor
        (:then
          (Development|PrintString "overlapping player"))
        (:CastFailed
          (bind _asbp_koopa (Utilities|Casting|CastToBP_Koopa OtherActor))
          (Actor|DestroyActor _asbp_koopa)
          (goto _label))))))

(event EventBeginPlay
  (Utilities|FlowControl|Sequence
    (:then_1
      (Utilities|FlowControl|Delay 4.0)
      (Actor|DestroyActor))))

(fn ConstructionScript)