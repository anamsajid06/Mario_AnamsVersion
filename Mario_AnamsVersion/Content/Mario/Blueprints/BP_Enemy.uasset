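; BP_Enemy is a Mario-style walking enemy that can be killed or hurt the player.
; It moves constantly along the Y axis, reversing via a FlipFlop on each hit.
; BoxCollision overlap by the player triggers death: collisions removed, movement stopped, capsule squashed, actor destroyed after a delay.
; BoxCollision2 overlap damages the player, or, if not big, shows the lost widget and reloads the level before dealing damage.
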(event OnComponentBeginOverlap(BoxCollision)
  (params (OverlappedComponent :type Primitive%20Component%20Object%20Reference) (OtherActor :type Actor%20Object%20Reference) (OtherComp :type Primitive%20Component%20Object%20Reference) (OtherBodyIndex :type Integer) (bFromSweep :type Boolean) (SweepResult :type Hit%20Result%20Structure%20%28by%20ref%29))
  ;[1 1 1] Enemy Death
  (Utilities|EnemyDeath OtherActor))

(event OnComponentBeginOverlap(BoxCollision2)
  (params (OverlappedComponent :type Primitive%20Component%20Object%20Reference) (OtherActor :type Actor%20Object%20Reference) (OtherComp :type Primitive%20Component%20Object%20Reference) (OtherBodyIndex :type Integer) (bFromSweep :type Boolean) (SweepResult :type Hit%20Result%20Structure%20%28by%20ref%29))
  ;[1 1 1] Player Damage
  (bind _asbp_third_person_character (Utilities|Casting|CastToBP_ThirdPersonCharacter OtherActor))
  (Utilities|FlowControl|Sequence
    (:then_0
      (if (Variables|/Game/ThirdPerson/Blueprints/BP_ThirdPersonCharacter.BP_ThirdPersonCharacter_C|GetbIsBig _asbp_third_person_character)
        (Development|PrintString (Utilities|String|ToString(Boolean) (Variables|/Game/ThirdPerson/Blueprints/BP_ThirdPersonCharacter.BP_ThirdPersonCharacter_C|GetbIsBig _asbp_third_person_character)))
        (else
          (Development|PrintString (Utilities|String|ToString(Boolean) (Variables|/Game/ThirdPerson/Blueprints/BP_ThirdPersonCharacter.BP_ThirdPersonCharacter_C|GetbIsBig _asbp_third_person_character)))
          ;[1 1 1] Lost Widget
          (bind _returnvalue (UserInterface|CreateWidget "/Game/Mario/Blueprints/BP_Lost.BP_Lost_C"))
          (UserInterface|Viewport|AddtoViewport _returnvalue 0)
          (Utilities|FlowControl|Delay 3.0)
          (bind _returnvalue_2 (Game|GetCurrentLevelName true))
          (Game|OpenLevel(byName) (Utilities|String|StringToName _returnvalue_2)))))
    (:then_1
      (Default|DealDamage _asbp_third_person_character))))

(event EventTick
  (params (DeltaSeconds :type Float%20%28single-precision%29))
  ;[1 1 1] Movement
  (Pawn|Input|AddMovementInput (Variables|Default|GetWorld%20Direction) 0.5 false))

(event Collision|EventHit
  (params (MyComp :type Primitive%20Component%20Object%20Reference) (Other :type Actor%20Object%20Reference) (OtherComp :type Primitive%20Component%20Object%20Reference) (bSelfMoved :type Boolean) (HitLocation :type Vector :default "0, 0, 0") (HitNormal :type Vector :default "0, 0, 0") (NormalImpulse :type Vector :default "0, 0, 0") (Hit :type Hit%20Result%20Structure%20%28by%20ref%29))
  ;[1 1 1] Change Direction
  (Utilities|FlowControl|FlipFlop
    (:A
      (Variables|Default|SetWorld%20Direction "0,1.000000, 0"))
    (:B
      (Variables|Default|SetWorld%20Direction "0,-1.000000, 0"))))

(fn ConstructionScript)