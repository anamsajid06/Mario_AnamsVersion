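; BP_Koopa is a Mario-style Koopa enemy that patrols along the Y axis with a looping walk animation.
; Tick drives movement, and each Hit flips direction and mesh yaw through a FlipFlop.
; Player overlap with DeathCollision bounces the character and replaces the Koopa with a BP_Koopa_Shell.
; DamageCollision overlap damages the player, briefly disabling both triggers; lost-screen and level-restart logic is unconnected.
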(event OnComponentBeginOverlap(DeathCollision)
  (params (OverlappedComponent :type Primitive%20Component%20Object%20Reference) (OtherActor :type Actor%20Object%20Reference) (OtherComp :type Primitive%20Component%20Object%20Reference) (OtherBodyIndex :type Integer) (bFromSweep :type Boolean) (SweepResult :type Hit%20Result%20Structure%20%28by%20ref%29))
  ;[1 1 1] Death
  (bind _asbp_third_person_character (Utilities|Casting|CastToBP_ThirdPersonCharacter OtherActor))
  (CallFunction|Die _asbp_third_person_character))

(event OnComponentBeginOverlap(DamageCollision)
  (params (OverlappedComponent :type Primitive%20Component%20Object%20Reference) (OtherActor :type Actor%20Object%20Reference) (OtherComp :type Primitive%20Component%20Object%20Reference) (OtherBodyIndex :type Integer) (bFromSweep :type Boolean) (SweepResult :type Hit%20Result%20Structure%20%28by%20ref%29))
  ;[1 1 1] Cause Damage to Player
  (bind _asbp_third_person_character (Utilities|Casting|CastToBP_ThirdPersonCharacter OtherActor))
  (Collision|SetCollisionEnabled (Variables|Default|GetDeathCollision) "NoCollision")
  (Default|DealDamage _asbp_third_person_character)
  (Utilities|FlowControl|Delay 2.0)
  (Collision|SetCollisionEnabled (Variables|Default|GetDeathCollision) "QueryOnly"))

(event EventBeginPlay
  ;[1 1 1] Walk Animation
  (Components|Animation|PlayAnimation (Variables|Character|GetMesh) "/Game/Mario/Assets/Koopa/Animations/Walk.Walk" true))

(event EventTick
  (params (DeltaSeconds :type Float%20%28single-precision%29))
  ;[1 1 1] Movement
  (Pawn|Input|AddMovementInput (Variables|Default|GetWorld%20Direction) 0.1 false))

(event Collision|EventHit
  (params (MyComp :type Primitive%20Component%20Object%20Reference) (Other :type Actor%20Object%20Reference) (OtherComp :type Primitive%20Component%20Object%20Reference) (bSelfMoved :type Boolean) (HitLocation :type Vector :default "0, 0, 0") (HitNormal :type Vector :default "0, 0, 0") (NormalImpulse :type Vector :default "0, 0, 0") (Hit :type Hit%20Result%20Structure%20%28by%20ref%29))
  ;[1 1 1] Change Direction on Hit
  (Utilities|FlowControl|FlipFlop
    (:A
      (Variables|Default|SetWorld%20Direction "0,1.000000, 0")
      (Transformation|SetRelativeRotation (Variables|Character|GetMesh) (Math|Rotator|MakeRotator 0.0 0.0 0.0) false false))
    (:B
      (Variables|Default|SetWorld%20Direction "0,-1.000000, 0")
      (Transformation|SetRelativeRotation (Variables|Character|GetMesh) "0,180.000000, 0" false false))))

(fn ConstructionScript)

(fn Die
  (params (Character :type BP%20Third%20Person%20Character%20Object%20Reference))
  (bind _capsulecomponent (Variables|Collision|GetCapsuleComponent))
  (bind _returnvalue (Transformation|GetWorldTransform _capsulecomponent))
  (Components|DestroyComponent (Variables|Default|GetDeathCollision))
  (Default|ForceJump Character)
  (Pawn|Components|CharacterMovement|DisableMovement (Variables|Character|GetCharacterMovement))
  (Game|SpawnActorfromClass "/Game/Mario/Blueprints/Enemies/BP_Koopa_Shell.BP_Koopa_Shell_C" (Math|Transform|MakeTransform (Math|Vector|MakeVector (.x (.location _returnvalue)) (.y (.location _returnvalue)) 74.0) (.rotation _returnvalue) (.scale _returnvalue)) "Undefined" 0 0)
  (Actor|DestroyActor))