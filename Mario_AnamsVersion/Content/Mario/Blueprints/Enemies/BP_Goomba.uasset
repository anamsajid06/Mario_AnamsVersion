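; BP_Goomba is a Mario-style enemy that walks constantly along the Y axis, flipping direction on each hit via a FlipFlop.
; Overlapping its DeathCollider with the third-person character removes both colliders, forces the player to jump, spawns an actor at a fixed height and destroys the Goomba.
; Overlapping its DamageCollider damages the player and disables both colliders for a short delay to prevent repeat hits.
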(event OnComponentBeginOverlap(DeathCollider)
  (params (OverlappedComponent :type Primitive%20Component%20Object%20Reference) (OtherActor :type Actor%20Object%20Reference) (OtherComp :type Primitive%20Component%20Object%20Reference) (OtherBodyIndex :type Integer) (bFromSweep :type Boolean) (SweepResult :type Hit%20Result%20Structure%20%28by%20ref%29))
  ;[1 1 1] Enemy Death
  (bind _asbp_third_person_character (Utilities|Casting|CastToBP_ThirdPersonCharacter OtherActor))
  (Utilities|EnemyDeath _asbp_third_person_character))

(event OnComponentBeginOverlap(DamageCollider)
  (params (OverlappedComponent :type Primitive%20Component%20Object%20Reference) (OtherActor :type Actor%20Object%20Reference) (OtherComp :type Primitive%20Component%20Object%20Reference) (OtherBodyIndex :type Integer) (bFromSweep :type Boolean) (SweepResult :type Hit%20Result%20Structure%20%28by%20ref%29))
  ;[1 1 1] Player Damage
  (bind _asbp_third_person_character (Utilities|Casting|CastToBP_ThirdPersonCharacter OtherActor))
  (Collision|SetCollisionEnabled (Variables|Default|GetDamageCollider) "NoCollision")
  (Default|DealDamage _asbp_third_person_character)
  (Utilities|FlowControl|Delay 2.0)
  (Collision|SetCollisionEnabled (Variables|Default|GetDamageCollider) "QueryOnly"))

(event EventTick
  (params (DeltaSeconds :type Float%20%28single-precision%29))
  ;[1 1 1] Movement
  (Pawn|Input|AddMovementInput (Variables|Default|GetWorld%20Direction) 0.5 false))

(event Collision|EventHit
  (params (MyComp :type Primitive%20Component%20Object%20Reference) (Other :type Actor%20Object%20Reference) (OtherComp :type Primitive%20Component%20Object%20Reference) (bSelfMoved :type Boolean) (HitLocation :type Vector :default "0, 0, 0") (HitNormal :type Vector :default "0, 0, 0") (NormalImpulse :type Vector :default "0, 0, 0") (Hit :type Hit%20Result%20Structure%20%28by%20ref%29))
  ;[1 1 1] Change Direction
  (Utilities|FlowControl|FlipFlop
    (:A
      (Variables|Default|SetWorld%20Direction "0,1.000000, 0"))
    (:B
      (Variables|Default|SetWorld%20Direction "0,-1.000000, 0"))))

(fn ConstructionScript)