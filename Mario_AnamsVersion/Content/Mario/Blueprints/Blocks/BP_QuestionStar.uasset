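; Question block in a Mario-style game that releases a BP_Star when the player character touches its collision box.
; The first overlap destroys the box, making the block single-use, then bumps the root component upward.
; It spawns the star at StarSpawnPoint with its default controller, then lowers the block after a short delay.
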(event OnComponentBeginOverlap(BoxCollision)
  (params (OverlappedComponent :type Primitive%20Component%20Object%20Reference) (OtherActor :type Actor%20Object%20Reference) (OtherComp :type Primitive%20Component%20Object%20Reference) (OtherBodyIndex :type Integer) (bFromSweep :type Boolean) (SweepResult :type Hit%20Result%20Structure%20%28by%20ref%29))
  (bind _defaultsceneroot (Variables|Default|GetDefaultSceneRoot))
  (bind _defaultsceneroot_2 (Variables|Default|GetDefaultSceneRoot))
  (Utilities|Casting|CastToBP_ThirdPersonCharacter OtherActor)
  (Components|DestroyComponent (Variables|Default|GetBoxCollision))
  (Components|MoveComponentTo _defaultsceneroot_2 (+ (Variables|/Script/Engine.SceneComponent|GetRelativeLocation _defaultsceneroot_2) "0,0,30.000000") "0, 0, 0" false false 0.1 false)
  (bind _returnvalue (Game|SpawnActorfromClass "/Game/Mario/Blueprints/Pickups/BP_Star.BP_Star_C" (Math|Transform|MakeTransform (Transformation|GetWorldLocation (Variables|Default|GetStarSpawnPoint)) "0, 0, 0" "1.000000,1.000000,1.000000") "Undefined" 0 0))
  (Pawn|SpawnDefaultController _returnvalue)
  (Utilities|FlowControl|Delay 0.2)
  (Components|MoveComponentTo _defaultsceneroot (+ (Variables|/Script/Engine.SceneComponent|GetRelativeLocation _defaultsceneroot) "0,0,-30.000000") "0, 0, 0" false false 0.1 false))

(fn ConstructionScript)